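; Enemy spawner actor that periodically spawns AI enemies inside a box volume.
; On BeginPlay a looping timer fires SpawnEnemy at the SpawnFrequency interval.
; SpawnEnemy switches on WhatToSpawn to spawn either a shooter or an exploding enemy at a random point within the SpawnVolume bounds.
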(event Custom|SpawnEnemy
  (bind _spawnvolume (Variables|Default|GetSpawnVolume))
  (bind _returnvalue (Components|Box|GetScaledBoxExtent _spawnvolume))
  (bind _returnvalue_2 (Transformation|GetWorldLocation _spawnvolume))
  (bind _returnvalue_3 (Math|Random|RandomPointinBoundingBox _returnvalue_2 _returnvalue))
  (switch Utilities|FlowControl|Switch|SwitchonEnemyEnum (Variables|Default|GetWhatToSpawn)
    (:NewEnumerator0
      (AI|SpawnAIFromClass "/Game/Enemies/BP_ShooterEnemy.BP_ShooterEnemy_C" 0 _returnvalue_3 "0, 0, 0" false))
    (:NewEnumerator1
      (AI|SpawnAIFromClass "/Game/Enemies/BP_ExplodingEnemy.BP_ExplodingEnemy_C" 0 _returnvalue_3 "0, 0, 0" false))))

(event EventBeginPlay
  (Utilities|Time|SetTimerbyFunctionName 0 "SpawnEnemy" (Variables|Default|GetSpawnFrequency) true))

(fn ConstructionScript)