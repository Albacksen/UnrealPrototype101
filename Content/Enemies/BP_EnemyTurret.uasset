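; BP_EnemyTurret is a stationary enemy turret that tracks the player and fires projectiles at a steady rate.
; On BeginPlay, two looping timers call LookAtPlayer and Shoot by function name.
; LookAtPlayer rotates the whole actor toward player pawn 0 with a look-at rotation, updated on a short timer instead of Tick.
; Shoot spawns a BP_EnemyProjectile at the SpawnProjectilePoint0 component's world location and rotation.
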(event Custom|LookAtPlayer
  (Transformation|SetActorRotation (Math|Rotator|FindLookatRotation (Transformation|GetActorLocation self) (Transformation|GetActorLocation (Game|Player|GetPlayerPawn 0)))))

(event Custom|Shoot
  (bind _spawnprojectilepoint_0 (Variables|Default|GetSpawnProjectilePoint_0))
  (Game|SpawnActorfromClass "/Game/Enemies/BP_EnemyProjectile.BP_EnemyProjectile_C" (Math|Transform|MakeTransform (Transformation|GetWorldLocation _spawnprojectilepoint_0) (Transformation|GetWorldRotation _spawnprojectilepoint_0)) "Undefined" 0 0))

(event EventBeginPlay
  (Utilities|Time|SetTimerbyFunctionName 0 "LookAtPlayer" 0.1 true)
  (Utilities|Time|SetTimerbyFunctionName 0 "Shoot" 1.0 true))

(fn ConstructionScript)