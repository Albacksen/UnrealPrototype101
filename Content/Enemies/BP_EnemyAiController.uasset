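; AI controller for patrolling enemies that runs the Enemy_BT behavior tree and reports whether the player is seen.
; On BeginPlay it casts its pawn to BP_Enemy and seeds the blackboard with that enemy's patrol path looping flag, wait time and a starting direction.
; AI Perception updates filter for TwinStickPawn and write the sensing result to the CanSeePlayer key.
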(event OnTargetPerceptionUpdated(AIPerception)
  (params (Actor :type Actor%20Object%20Reference) (Stimulus :type AI%20Stimulus%20Structure))
  (Utilities|Casting|CastToTwinStickPawn Actor)
  (AI|Components|Blackboard|SetValueasBool (AI|GetBlackboard 0) (Utilities|Name|MakeLiteralName "CanSeePlayer") (.bSuccessfullySensed (Utilities|Struct|BreakAIStimulus Stimulus))))

(event EventBeginPlay
  (bind _returnvalue (AI|GetBlackboard 0))
  (AI|RunBehaviorTree "/Game/Enemies/AI/Enemy/Enemy_BT.Enemy_BT")
  (bind _asbp_enemy (Utilities|Casting|CastToBP_Enemy (Pawn|GetControlledPawn)))
  (bind _output_get (Variables|Default|SetMyPawn _asbp_enemy))
  (AI|Components|Blackboard|SetValueasBool _returnvalue (Utilities|Name|MakeLiteralName "PathLooping") (Variables|/Game/Enemies/AI/Enemy/PatrolPath.PatrolPath_C|GetIsLooping (Variables|/Game/Enemies/AI/Enemy/BP_Enemy.BP_Enemy_C|GetPatrolPath _output_get)))
  (Class|BlackboardComponent|SetValueasInt (AI|GetBlackboard 0) (Utilities|Name|MakeLiteralName "Direction") 1)
  (AI|Components|Blackboard|SetValueasFloat _returnvalue (Utilities|Name|MakeLiteralName "WaitTime") (Variables|/Game/Enemies/AI/Enemy/PatrolPath.PatrolPath_C|GetWaitTime (Variables|/Game/Enemies/AI/Enemy/BP_Enemy.BP_Enemy_C|GetPatrolPath (Variables|Default|GetMyPawn)))))

(fn ConstructionScript)