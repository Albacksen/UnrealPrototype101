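; Exploding enemy Blueprint for a twin-stick shooter that can be shot down or detonate when the player gets close.
; Projectile hits lower HP; at zero it hides its meshes, activates the explosion and destroys itself after a short delay.
; The player entering Sphere1 starts a one-time delayed detonation, destroying the pawn if still inside the blast radius, tracked through begin/end overlap, then itself.
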(event OnComponentBeginOverlap(Sphere1)
  (params (OverlappedComponent :type Primitive%20Component%20Object%20Reference) (OtherActor :type Actor%20Object%20Reference) (OtherComp :type Primitive%20Component%20Object%20Reference) (OtherBodyIndex :type Integer) (bFromSweep :type Boolean) (SweepResult :type Hit%20Result%20Structure%20%28by%20ref%29))
  (bind _astwin_stick_pawn (Utilities|Casting|CastToTwinStickPawn OtherActor))
  (Utilities|FlowControl|DoOnce false
    (:Completed
      (Variables|Default|SetInsideBlastRadius true)
      (Utilities|FlowControl|Delay 1.0)
      (Rendering|SetVisibility (Variables|Default|GetCylinder_0) false false)
      (Components|Activation|Activate (Variables|Default|GetExplosion) false)
      (Utilities|FlowControl|Sequence
        (:then_0
          (if (Variables|Default|GetInsideBlastRadius)
            (Actor|DestroyActor _astwin_stick_pawn)
            (Development|PrintString "youdie")))
        (:then_1
          (Utilities|FlowControl|Delay 0.2)
          (Actor|DestroyActor)
          (Development|PrintString "medie"))))))

(event OnComponentEndOverlap(Sphere1)
  (params (OverlappedComponent :type Primitive%20Component%20Object%20Reference) (OtherActor :type Actor%20Object%20Reference) (OtherComp :type Primitive%20Component%20Object%20Reference) (OtherBodyIndex :type Integer))
  (Utilities|Casting|CastToTwinStickPawn OtherActor)
  (Variables|Default|SetInsideBlastRadius false))

(event Collision|EventHit
  (params (MyComp :type Primitive%20Component%20Object%20Reference) (Other :type Actor%20Object%20Reference) (OtherComp :type Primitive%20Component%20Object%20Reference) (bSelfMoved :type Boolean) (HitLocation :type Vector :default "0, 0, 0") (HitNormal :type Vector :default "0, 0, 0") (NormalImpulse :type Vector :default "0, 0, 0") (Hit :type Hit%20Result%20Structure%20%28by%20ref%29))
  (Utilities|Casting|CastToTwinStickProjectile Other)
  (bind _output_get (Variables|Default|SetHP (- (Variables|Default|GetHP) 1)))
  (if (<= _output_get 0)
    (Rendering|SetVisibility (Variables|Default|GetCylinder_0) false false)
    (Components|Activation|Activate (Variables|Default|GetExplosion) false)
    (Utilities|FlowControl|Delay 0.5)
    (Actor|DestroyActor)))

(fn ConstructionScript)