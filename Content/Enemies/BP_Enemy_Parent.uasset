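; Parent enemy Blueprint that turns to face player 0's pawn and dies when shot.
; BeginPlay starts looping timers for LookAtPlayer, which snaps the actor's rotation toward the player ten times a second, and for Shoot.
; A hit from a TwinStickProjectile destroys the enemy after a short delay.
; Shoot is an empty stub here, and the BP_EnemyProjectile spawn node is disconnected.
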(event Custom|LookAtPlayer
  (Transformation|SetActorRotation (Math|Rotator|FindLookatRotation (Transformation|GetActorLocation self) (Transformation|GetActorLocation (Game|Player|GetPlayerPawn 0)))))

(event Custom|Shoot
  ;[1 1 1] inactive
)

(event EventBeginPlay
  (Utilities|Time|SetTimerbyFunctionName 0 "LookAtPlayer" 0.1 true)
  (Utilities|Time|SetTimerbyFunctionName 0 "Shoot" 1.0 true))

(event Collision|EventHit
  (params (MyComp :type Primitive%20Component%20Object%20Reference) (Other :type Actor%20Object%20Reference) (OtherComp :type Primitive%20Component%20Object%20Reference) (bSelfMoved :type Boolean) (HitLocation :type Vector :default "0, 0, 0") (HitNormal :type Vector :default "0, 0, 0") (NormalImpulse :type Vector :default "0, 0, 0") (Hit :type Hit%20Result%20Structure%20%28by%20ref%29))
  (Utilities|Casting|CastToTwinStickProjectile Other)
  (Utilities|FlowControl|Delay 0.2)
  (Actor|DestroyActor))

(fn ConstructionScript)