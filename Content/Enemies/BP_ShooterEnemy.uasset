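; Shooter enemy that patrols assigned points or wanders the navmesh when none are set, and chases and shoots at the player.
; Looping timers run a line-of-sight and distance check that sets PlayerInRange, and spawn projectiles while it is true.
; Tick issues AI moves toward the player when in range or damaged, wraps the patrol index, and uses a DoOnce to resume patrol when sight is lost.
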(event Custom|Shoot
  (bind _spawnprojectilepoint_0 (Variables|Default|GetSpawnProjectilePoint_0))
  ;[1 1 1] Shoots Projectiles
  (if (Variables|Default|GetPlayerInRange)
    (Game|SpawnActorfromClass "/Game/Enemies/BP_EnemyProjectile.BP_EnemyProjectile_C" (Math|Transform|MakeTransform (Transformation|GetWorldLocation _spawnprojectilepoint_0) (Transformation|GetWorldRotation _spawnprojectilepoint_0)) "Undefined" 0 0)))

(event Custom|GoToNextPoint
  ;[1 1 1] What Point To move To
  (if (not (Variables|Default|GetPlayerInRange))
    (AI|AIMoveTo (AI|GetAIController self) "0, 0, 0" (Utilities|Array|Get(acopy) (Variables|Default|GetMoveToPoint) (Variables|Default|GetNextMoveToPoint)) -1.0 "Default" "Default" true true)))

(event Custom|LookingForPlayer
  ;[1 1 1] Looking At Player
  (bind _outhit (Collision|LineTraceByChannel (Transformation|GetWorldLocation (Variables|Default|GetHead)) (Transformation|GetActorLocation (Game|Player|GetPlayerPawn 0)) "TraceTypeQuery1" false 0 "None"))
  (if (Math|Boolean|ORBoolean (.bBlockingHit (Collision|BreakHitResult _outhit)) (> (Transformation|GetDistanceTo (Game|GetPlayerCharacter 0)) 1e+03) false)
    (Utilities|FlowControl|Delay 1.0)
    (Variables|Default|SetPlayerInRange false)
    (else
      (Variables|Default|SetPlayerInRange true))))

(event EventBeginPlay
  ;[1 1 1] BeginPlay
  (Utilities|Time|SetTimerbyFunctionName 0 "Shoot" 1.0 true)
  (if (> (Utilities|Array|Length (Variables|Default|GetMoveToPoint)) 0)
    (Utilities|Time|SetTimerbyFunctionName 0 "GoToNextPoint" 0.1)
    (else
      (Variables|Default|SetRandomMovement true)))
  (Utilities|Time|SetTimerbyFunctionName 0 "LookingForPlayer" 0.5 true))

(event EventTick
  (params (DeltaSeconds :type Float%20%28single-precision%29))
  (Utilities|FlowControl|Sequence
    (:then_0
      ;[1 1 1] Move To Player When Shot
      (if (Variables|Default|GetTakenDamage?)
        (if (not (Variables|Default|GetIsDead?)) :!label _label
          (AI|AIMoveTo self "0, 0, 0" (Game|GetPlayerController 0) 3e+02 false))))
    (:then_1
      (if (Variables|Default|GetPlayerInRange)
        (Utilities|FlowControl|Sequence
          (:then_0
            (goto _label))
          (:then_1
            (goto _label_2 Reset)))
        (else
          (Utilities|FlowControl|DoOnce false :!label _label_2
            (:Completed
              (CallFunction|GotoNextPoint))))))
    (:then_2
      (if (> (Variables|Default|GetNextMoveToPoint) (- (Utilities|Array|Length (Variables|Default|GetMoveToPoint)) 1))
        (Variables|Default|SetNextMoveToPoint 0)))
    (:then_3
      ;[1 1 1] Move To Random Location When No Point Is Assigned
      (if (Variables|Default|GetRandomMovement)
        (if (not (Variables|Default|GetPlayerInRange))
          (Utilities|FlowControl|Delay 5.0)
          (AI|AIMoveTo self (.RandomLocation (Class|NavigationSystemV1|GetRandomPointinNavigableRadius (Transformation|GetWorldLocation (Variables|Character|GetMesh self)) 1e+03 0 0)) 0 1.0 false))))))

(fn ConstructionScript)