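; Enemy character that takes damage, attacks with projectiles or a melee montage, and shows its health on a widget bar updated each Tick.
; Damage briefly sets the blackboard's CanSeePlayer flag, alerting the AI even without a sighting.
; At zero health it sets IsDead, enables mesh physics, rolls once for an ammo or health pickup drop, and destroys itself after a short delay.
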(event EventShootingAttack
  (bind _projectilespawnpoint (Variables|Default|GetProjectileSpawnPoint))
  (Game|SpawnActorfromClass "/Game/Enemies/BP_EnemyProjectile.BP_EnemyProjectile_C" (Math|Transform|MakeTransform (Transformation|GetWorldLocation _projectilespawnpoint) (Transformation|GetWorldRotation _projectilespawnpoint) "1,1,1.000000") "Undefined" 0 0))

(event EventTakeDamage
  (params (DamageTaken :type Integer))
  (bind _capsulecomponent (Variables|Collision|GetCapsuleComponent))
  (bind _returnvalue (Transformation|GetWorldLocation _capsulecomponent))
  (bind _returnvalue_2 (Math|Conversions|ToTransform(Vector) _returnvalue))
  (Utilities|FlowControl|Sequence
    (:then_0
      (AI|Components|Blackboard|SetValueasBool (AI|GetBlackboard 0) (Utilities|Name|MakeLiteralName "CanSeePlayer") true)
      (Utilities|FlowControl|Delay 5.0)
      (AI|Components|Blackboard|SetValueasBool (AI|GetBlackboard 0) (Utilities|Name|MakeLiteralName "CanSeePlayer") false))
    (:then_1
      (bind _output_get (Variables|Default|SetHealth (- (Variables|Default|GetHealth) (Math|Conversions|ToFloat(Integer) DamageTaken))))
      (if (<= _output_get 0.0)
        (AI|Components|Blackboard|SetValueasBool (AI|GetBlackboard 0) (Utilities|Name|MakeLiteralName "IsDead") true)
        (Physics|SetSimulatePhysics (Variables|Character|GetMesh) true)
        (Utilities|FlowControl|Sequence
          (:then_0
            (Utilities|FlowControl|DoOnce false
              (:Completed
                (switch Utilities|FlowControl|Switch|SwitchonPickUpsDrop (Utilities|Enum|ByteToEnumPickUpsDrop (Math|Conversions|ToByte(Integer) (Math|Random|RandomIntegerinRange 0 5)))
                  (:NewEnumerator0
                    (Game|SpawnActorfromClass :Class "/Game/TwinStickBP/Blueprints/WeaponAndAmmo_BP/AmmoPickup_Weapon_01.AmmoPickup_Weapon_01_C" :SpawnTransform _returnvalue_2 :CollisionHandlingOverride "Undefined" :AmmoPickupAmount (Math|Random|RandomIntegerinRange 10 30) :Instigator 0))
                  (:NewEnumerator1
                    (Game|SpawnActorfromClass :Class "/Game/TwinStickBP/Blueprints/WeaponAndAmmo_BP/AmmoPickup_Weapon_02.AmmoPickup_Weapon_02_C" :SpawnTransform _returnvalue_2 :CollisionHandlingOverride "Undefined" :AmmoPickupAmount (Math|Random|RandomIntegerinRange 10 30) :Instigator 0))
                  (:NewEnumerator2
                    (Game|SpawnActorfromClass :Class "/Game/TwinStickBP/Blueprints/WeaponAndAmmo_BP/AmmoPickup_Weapon_03.AmmoPickup_Weapon_03_C" :SpawnTransform _returnvalue_2 :CollisionHandlingOverride "Undefined" :AmmoPickupAmount (Math|Random|RandomIntegerinRange 3 24) :Instigator 0))
                  (:NewEnumerator3
                    (Game|SpawnActorfromClass :Class "/Game/TwinStickBP/Blueprints/WeaponAndAmmo_BP/AmmoPickup_Weapon_04.AmmoPickup_Weapon_04_C" :SpawnTransform _returnvalue_2 :CollisionHandlingOverride "Undefined" :AmmoPickupAmount (Math|Random|RandomIntegerinRange 15 50) :Instigator 0))
                  (:NewEnumerator4
                    (Game|SpawnActorfromClass "/Game/TwinStickBP/Blueprints/Health_Pickup_Parent.Health_Pickup_Parent_C" _returnvalue_2 "Undefined" 0 (Math|Random|RandomIntegerinRange 3 10) 0))))))
          (:then_1
            (Utilities|FlowControl|Delay 2.0)
            (Actor|DestroyActor)))))))

(event EventBeginPlay
  (Variables|Default|SetHealth (Variables|Default|GetMaxHealth))
  (bind _asenemy_health (Utilities|Casting|CastToEnemyHealth (UserInterface|GetUserWidgetObject (Variables|Default|GetHealth%20Bar)))))

(event EventTick
  (params (DeltaSeconds :type Float%20%28single-precision%29))
  (Progress|SetPercent (Variables|/Game/Enemies/EnemyHealth.EnemyHealth_C|GetProgressBar_65 (stale EventBeginPlay _asenemy_health)) (/ (Variables|Default|GetHealth) (Variables|Default|GetMaxHealth))))

(event EventMeleeAttack
  (Animation|Montage|PlayMontage (Variables|Character|GetMesh) "/Game/Enemies/Attack_PrimaryA_Montage.Attack_PrimaryA_Montage"))

(fn ConstructionScript)