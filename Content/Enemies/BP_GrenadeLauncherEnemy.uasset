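; BP_GrenadeLauncherEnemy is an enemy that fires grenades and can be destroyed by twin-stick projectiles.
; A looping timer started on BeginPlay spawns BP_Grenade at the spawn point component every second.
; Hits from TwinStickProjectile reduce HP; at zero it hides its cylinder and sphere meshes, activates a particle effect, and destroys itself after a short delay.
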(event Custom|Shoot
  (bind _spawnprojectilepoint_0 (Variables|Default|GetSpawnProjectilePoint_0))
  (Game|SpawnActorfromClass "/Game/Enemies/BP_Grenade.BP_Grenade_C" (Math|Transform|MakeTransform (Transformation|GetWorldLocation _spawnprojectilepoint_0) (Transformation|GetWorldRotation _spawnprojectilepoint_0)) "Undefined" 0 0))

(event EventBeginPlay
  (Utilities|Time|SetTimerbyFunctionName 0 "Shoot" 1.0 true))

(event Collision|EventHit
  (params (MyComp :type Primitive%20Component%20Object%20Reference) (Other :type Actor%20Object%20Reference) (OtherComp :type Primitive%20Component%20Object%20Reference) (bSelfMoved :type Boolean) (HitLocation :type Vector :default "0, 0, 0") (HitNormal :type Vector :default "0, 0, 0") (NormalImpulse :type Vector :default "0, 0, 0") (Hit :type Hit%20Result%20Structure%20%28by%20ref%29))
  (Utilities|Casting|CastToTwinStickProjectile Other)
  (bind _output_get (Variables|Default|SetHP (- (Variables|Default|GetHP) 1)))
  (if (<= _output_get 0)
    (Rendering|SetVisibility (Variables|Default|GetCylinder_0) false false)
    (Components|Activation|Activate (Variables|Default|GetParticleSystem) false)
    (Utilities|FlowControl|Delay 0.5)
    (Actor|DestroyActor)))

(fn ConstructionScript)