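; BP_BlockPassage is a level trap that seals a passage with four stone meshes when the TwinStickPawn enters its trigger.
; The stones start hidden with collision disabled on BeginPlay.
; Trigger overlap by the pawn plays a world camera shake at its location, and if the overlapping component is its capsule, the stones become visible and solid.
; Nothing in the graph hides them again or prevents the shake from repeating.
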(event OnComponentBeginOverlap(Trigger)
  (params (OverlappedComponent :type Primitive%20Component%20Object%20Reference) (OtherActor :type Actor%20Object%20Reference) (OtherComp :type Primitive%20Component%20Object%20Reference) (OtherBodyIndex :type Integer) (bFromSweep :type Boolean) (SweepResult :type Hit%20Result%20Structure%20%28by%20ref%29))
  (bind _stone (Variables|Default|GetStone))
  (bind _astwin_stick_pawn (Utilities|Casting|CastToTwinStickPawn OtherActor))
  (Camera|PlayWorldCameraShake "/Game/LevelContent/MyCameraShake.MyCameraShake_C" (Transformation|GetActorLocation _astwin_stick_pawn) 1e+01 5e+02 2.0 true)
  (if (== OtherComp (Variables|/Script/Engine.Character|GetCapsuleComponent _astwin_stick_pawn))
    (Collision|SetCollisionEnabled _stone "QueryAndPhysics")
    (Rendering|SetVisibility _stone true false)))

(event EventBeginPlay
  (bind _stone (Variables|Default|GetStone))
  (Rendering|SetVisibility _stone false false)
  (Collision|SetCollisionEnabled _stone "NoCollision"))

(fn ConstructionScript)