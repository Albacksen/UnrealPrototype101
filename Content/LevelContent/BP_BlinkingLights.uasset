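; BP_BlinkingLights is a light actor that animates a point light with a selectable blink pattern.
; On BeginPlay, LightPattern picks one of four timelines, including a Steady Blink option, whose curve is multiplied by Intensity to drive brightness.
; BeginPlay also applies the Color variable to the light.
; The StopLights event hides the light without stopping the running timeline.
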(event Custom|StopLights
  (Rendering|SetVisibility (Variables|Default|GetPointLight) false false))

(event EventBeginPlay
  (bind _intensity (Variables|Default|GetIntensity))
  (Utilities|FlowControl|Sequence
    (:then_0
      (switch Utilities|FlowControl|Switch|SwitchonLightPatterns (Variables|Default|GetLight%20Pattern)
        (:NewEnumerator0
          (bind _lightintensity (Timeline|LightIntensity PlayFromStart)
            (:Update
              (Rendering|Components|Light|SetIntensity (Variables|Default|GetPointLight) (* _lightintensity _intensity)))))
        (:NewEnumerator1
          (bind _lightintensity_2 (Timeline|Timeline_0 PlayFromStart)
            (:Update
              (Rendering|Components|Light|SetIntensity (Variables|Default|GetPointLight) (* _lightintensity_2 _intensity)))))
        (:NewEnumerator2
          (bind _lightintensity_3 (Timeline|Timeline_1 PlayFromStart)
            (:Update
              (Rendering|Components|Light|SetIntensity (Variables|Default|GetPointLight) (* _lightintensity_3 _intensity)))))
        (:NewEnumerator3
          (bind _lightintensity_4 (Timeline|Timeline_2 PlayFromStart)
            (:Update
              (Rendering|Components|Light|SetIntensity (Variables|Default|GetPointLight) (* _lightintensity_4 _intensity)))))))
    (:then_1
      (Rendering|Components|Light|SetLightColor (Variables|Default|GetPointLight) (Variables|Default|GetColor) true))))

(fn ConstructionScript)