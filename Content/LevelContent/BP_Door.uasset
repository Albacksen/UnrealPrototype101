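; BP_Door is a sliding double door that opens for the TwinStickPawn, either on proximity alone or once unlocked through keys.
; In Keys mode a looping timer polls the Keys array and unlocks when the last element is no longer valid, without checking the others.
; When unlocked, capsule overlap with the Box plays or reverses a timeline that moves each panel along its own spline, keeping rotation and scale.
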(event OnComponentBeginOverlap(Box)
  (params (OverlappedComponent :type Primitive%20Component%20Object%20Reference) (OtherActor :type Actor%20Object%20Reference) (OtherComp :type Primitive%20Component%20Object%20Reference) (OtherBodyIndex :type Integer) (bFromSweep :type Boolean) (SweepResult :type Hit%20Result%20Structure%20%28by%20ref%29))
  (bind _spline1 (Variables|Default|GetSpline1))
  (bind _door1 (Variables|Default|GetDoor1))
  (bind _door (Variables|Default|GetDoor))
  (bind _spline (Variables|Default|GetSpline))
  (bind _astwin_stick_pawn (Utilities|Casting|CastToTwinStickPawn OtherActor))
  (if (== (Variables|/Script/Engine.Character|GetCapsuleComponent _astwin_stick_pawn) OtherComp)
    (if (Variables|Default|GetDoorCanOpen)
      (bind _dooropening (Timeline|DoorOpening Play)
        (:Update
          (Utilities|FlowControl|Sequence
            (:then_0
              (Transformation|SetWorldTransform (Variables|Default|GetDoor1) (Math|Transform|MakeTransform (Spline|GetLocationatDistanceAlongSpline _spline (* (Spline|GetSplineLength _spline) _dooropening) "World") (Transformation|GetWorldRotation _door1) (Transformation|GetWorldScale _door1)) false false))
            (:then_1
              (Transformation|SetWorldTransform (Variables|Default|GetDoor) (Math|Transform|MakeTransform (Spline|GetLocationatDistanceAlongSpline _spline1 (* (Spline|GetSplineLength _spline1) _dooropening) "World") (Transformation|GetWorldRotation _door) (Transformation|GetWorldScale _door)) false false))))))))

(event OnComponentEndOverlap(Box)
  (params (OverlappedComponent :type Primitive%20Component%20Object%20Reference) (OtherActor :type Actor%20Object%20Reference) (OtherComp :type Primitive%20Component%20Object%20Reference) (OtherBodyIndex :type Integer))
  (bind _spline1 (Variables|Default|GetSpline1))
  (bind _door1 (Variables|Default|GetDoor1))
  (bind _door (Variables|Default|GetDoor))
  (bind _spline (Variables|Default|GetSpline))
  (bind _astwin_stick_pawn (Utilities|Casting|CastToTwinStickPawn OtherActor))
  (if (== (Variables|/Script/Engine.Character|GetCapsuleComponent _astwin_stick_pawn) OtherComp)
    (if (Variables|Default|GetDoorCanOpen)
      (bind _dooropening (Timeline|DoorOpening Reverse)
        (:Update
          (Utilities|FlowControl|Sequence
            (:then_0
              (Transformation|SetWorldTransform (Variables|Default|GetDoor1) (Math|Transform|MakeTransform (Spline|GetLocationatDistanceAlongSpline _spline (* (Spline|GetSplineLength _spline) _dooropening) "World") (Transformation|GetWorldRotation _door1) (Transformation|GetWorldScale _door1)) false false))
            (:then_1
              (Transformation|SetWorldTransform (Variables|Default|GetDoor) (Math|Transform|MakeTransform (Spline|GetLocationatDistanceAlongSpline _spline1 (* (Spline|GetSplineLength _spline1) _dooropening) "World") (Transformation|GetWorldRotation _door) (Transformation|GetWorldScale _door)) false false))))))))

(event Custom|KeyEvent
  (for _array_element (Variables|Default|GetKeys)
    _)
  (if (not (Utilities|IsValid _array_element))
    (Variables|Default|SetDoorCanOpen true)))

(event EventBeginPlay
  (switch Utilities|FlowControl|Switch|SwitchonDoorOptions (Variables|Default|GetDoorOptions)
    (:NewEnumerator0
      (Variables|Default|SetDoorCanOpen true))
    (:NewEnumerator1
      (Utilities|Time|SetTimerbyFunctionName 0 "KeyEvent" 0.2 true)
      (CallFunction|KeyEvent))))

(fn ConstructionScript)