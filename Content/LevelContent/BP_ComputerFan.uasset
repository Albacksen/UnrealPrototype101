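; BP_ComputerFan is an interactable fan that, once switched on, activates a referenced computer.
; The Interact event runs once through a DoOnce and calls Activation on the Computer reference.
; It then spins the fan by setting the RotatingMovement rate, plays a ventilation sound at the Cylinder's location and turns the referenced Light's point light green.
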(event EventInteract
  (Utilities|FlowControl|DoOnce false
    (:Completed
      (Default|Activation (Variables|Default|GetComputer))
      (Variables|/Script/Engine.RotatingMovementComponent|SetRotationRate (Variables|Default|GetRotatingMovement) "0,800.000000,0.000000")
      (Audio|PlaySoundatLocation "/Game/Audio/Ventilation.Ventilation" (Transformation|GetWorldLocation (Variables|Default|GetCylinder)) "0, 0, 0" 1.0 1.0 0.0 0 0 0)
      (Rendering|Components|Light|SetLightColor (Variables|/Game/LevelContent/BP_BlinkingLights.BP_BlinkingLights_C|GetPointLight (Variables|Default|GetLight)) "(R=0.088937,G=1.000000,B=0.000000,A=1.000000)" true))))

(fn ConstructionScript)