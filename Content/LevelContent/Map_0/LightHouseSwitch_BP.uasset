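; LightHouseSwitch_BP is an interactable switch in Map_0 that sets a referenced Boat moving and shows a short timed camera sequence.
; On Interact it calls Move on the Boat, disables player input and blends the view target to the switch itself.
; After a fixed delay, it blends the view back to the player character and re-enables input.
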(event EventInteract
  (bind _returnvalue (Game|GetPlayerController 0))
  (bind _returnvalue_2 (Game|GetPlayerController 0))
  (Default|Move (Variables|Default|GetBoat))
  (Input|DisableInput _returnvalue_2 _returnvalue_2)
  (Game|Player|SetViewTargetwithBlend (Game|GetPlayerController 0) self 2.0 "VTBlend_Linear" 0.0 false)
  (Utilities|FlowControl|Delay 1e+01)
  (Game|Player|SetViewTargetwithBlend (Game|GetPlayerController 0) (Game|GetPlayerCharacter 0) 2.0 "VTBlend_Linear" 0.0 false)
  (Input|EnableInput _returnvalue _returnvalue))

(fn ConstructionScript)