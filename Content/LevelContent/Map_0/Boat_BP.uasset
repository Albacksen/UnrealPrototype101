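; Boat Blueprint for Map_0 that moves along a spline and acts as a level exit to Map_01.
; The Move event, not called within this Blueprint, plays a timeline that sets the Cube's world location by distance along the spline.
; Separately, when a TwinStickPawn's capsule overlaps the Box, the camera fades out and Map_01 opens after a short delay.
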(event OnComponentBeginOverlap(Box)
  (params (OverlappedComponent :type Primitive%20Component%20Object%20Reference) (OtherActor :type Actor%20Object%20Reference) (OtherComp :type Primitive%20Component%20Object%20Reference) (OtherBodyIndex :type Integer) (bFromSweep :type Boolean) (SweepResult :type Hit%20Result%20Structure%20%28by%20ref%29))
  (bind _astwin_stick_pawn (Utilities|Casting|CastToTwinStickPawn OtherActor))
  (if (== OtherComp (Variables|/Script/Engine.Character|GetCapsuleComponent _astwin_stick_pawn))
    (CameraFades|StartCameraFade :self (Game|GetPlayerCameraManager _astwin_stick_pawn) :ToAlpha 1.0 :Duration 3.0)
    (Utilities|FlowControl|Delay 3.5)
    (Game|OpenLevel(byName) "Map_01")))

(event Custom|Move
  (bind _newtrack_0 (Timeline|Movement PlayFromStart)
    (:Update
      (bind _output_get (Variables|Default|SetAlpha _newtrack_0))
      (Transformation|SetWorldLocation (Variables|Default|GetCube) (Spline|GetLocationatDistanceAlongSpline (Variables|Default|GetSpline) (Math|Float|Lerp _output_get (Spline|GetSplineLength (Variables|Default|GetSpline)) (Variables|Default|GetAlpha)) "World") false false))))

(fn ConstructionScript)