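; BP_LevelStream is a trigger actor that streams a named sublevel in and out as a TwinStickPawn passes through it.
; Overlapping the Load component loads the level and makes it visible, while overlapping the UnLoad component unloads it, both as blocking operations.
; Both triggers respond only to the pawn's capsule component, so its other components do not fire them.
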(event OnComponentBeginOverlap(Load)
  (params (OverlappedComponent :type Primitive%20Component%20Object%20Reference) (OtherActor :type Actor%20Object%20Reference) (OtherComp :type Primitive%20Component%20Object%20Reference) (OtherBodyIndex :type Integer) (bFromSweep :type Boolean) (SweepResult :type Hit%20Result%20Structure%20%28by%20ref%29))
  (bind _astwin_stick_pawn (Utilities|Casting|CastToTwinStickPawn OtherActor))
  (if (== (Variables|/Script/Engine.Character|GetCapsuleComponent _astwin_stick_pawn) OtherComp)
    (Game|LoadStreamLevel(byName) (Variables|Default|GetLevelName) true true)))

(event OnComponentBeginOverlap(UnLoad)
  (params (OverlappedComponent :type Primitive%20Component%20Object%20Reference) (OtherActor :type Actor%20Object%20Reference) (OtherComp :type Primitive%20Component%20Object%20Reference) (OtherBodyIndex :type Integer) (bFromSweep :type Boolean) (SweepResult :type Hit%20Result%20Structure%20%28by%20ref%29))
  (bind _astwin_stick_pawn (Utilities|Casting|CastToTwinStickPawn OtherActor))
  (if (== (Variables|/Script/Engine.Character|GetCapsuleComponent _astwin_stick_pawn) OtherComp)
    (Game|UnloadStreamLevel(byName) (Variables|Default|GetLevelName) true)))

(event EventBeginPlay)

(event Collision|EventActorBeginOverlap
  (params (OtherActor :type Actor%20Object%20Reference)))

(event EventTick
  (params (DeltaSeconds :type Float%20%28single-precision%29)))

(fn ConstructionScript)