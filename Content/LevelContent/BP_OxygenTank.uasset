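; BP_OxygenTank is a level pickup station that refills a TwinStickPawn's Oxygen to full when Interact fires while the pawn is in range.
; Box overlaps with the pawn's capsule open and close a Gate that lets Interact through, and also set CanTakeOxygen.
; Tick shows OxygenLevel on a UI_OxygenTank widget bar.
; The TakeOxygen event is empty and the tank-draining logic is disconnected, so refills never lower OxygenLevel.
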(event OnComponentBeginOverlap(Box)
  (params (OverlappedComponent :type Primitive%20Component%20Object%20Reference) (OtherActor :type Actor%20Object%20Reference) (OtherComp :type Primitive%20Component%20Object%20Reference) (OtherBodyIndex :type Integer) (bFromSweep :type Boolean) (SweepResult :type Hit%20Result%20Structure%20%28by%20ref%29))
  (bind _astwin_stick_pawn (Utilities|Casting|CastToTwinStickPawn OtherActor))
  (if (== OtherComp (Variables|/Script/Engine.Character|GetCapsuleComponent _astwin_stick_pawn))
    (Variables|Default|SetCanTakeOxygen true)
    (Utilities|FlowControl|Gate true) ; enters at Open
  ))

(event OnComponentEndOverlap(Box)
  (params (OverlappedComponent :type Primitive%20Component%20Object%20Reference) (OtherActor :type Actor%20Object%20Reference) (OtherComp :type Primitive%20Component%20Object%20Reference) (OtherBodyIndex :type Integer))
  (bind _astwin_stick_pawn (Utilities|Casting|CastToTwinStickPawn OtherActor))
  (if (== OtherComp (Variables|/Script/Engine.Character|GetCapsuleComponent _astwin_stick_pawn))
    (Variables|Default|SetCanTakeOxygen false)
    (Utilities|FlowControl|Gate true) ; enters at Close
  ))

(event Custom|TakeOxygen)

(event EventBeginPlay
  (bind _asui_oxygen_tank (Utilities|Casting|CastToUI_OxygenTank (UserInterface|GetUserWidgetObject (Variables|Default|GetWidget)))))

(event EventTick
  (params (DeltaSeconds :type Float%20%28single-precision%29))
  (Progress|SetPercent (Variables|/Game/UI/UI_OxygenTank.UI_OxygenTank_C|GetProgressBar_368 (stale EventBeginPlay _asui_oxygen_tank)) (/ (Variables|Default|GetOxygenLevel) 1e+02))
  (if (Variables|Default|GetCanTakeOxygen)
    (if (Variables|Default|GetTake)
      (CallFunction|TakeOxygen))))

(event EventInteract
  (Utilities|FlowControl|Gate true
    (:Exit
      (Variables|/Game/TwinStickBP/Blueprints/TwinStickPawn.TwinStickPawn_C|SetOxygen (stale OnComponentBeginOverlap(Box) _astwin_stick_pawn) 1e+02))))

(fn ConstructionScript)