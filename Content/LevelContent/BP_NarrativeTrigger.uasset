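; BP_NarrativeTrigger is a placed trigger volume that shows a narrative pop-up when the player walks into it.
; On box overlap by an actor tagged Player, it creates a UI_NarrativePopUp widget, fills it with its NarrativeText and adds it to the viewport.
; It then disables player pawn input and shows the mouse cursor.
; The end-overlap handler does nothing, and a leftover Gate node is unconnected.
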(event OnComponentBeginOverlap(Box)
  (params (OverlappedComponent :type Primitive%20Component%20Object%20Reference) (OtherActor :type Actor%20Object%20Reference) (OtherComp :type Primitive%20Component%20Object%20Reference) (OtherBodyIndex :type Integer) (bFromSweep :type Boolean) (SweepResult :type Hit%20Result%20Structure%20%28by%20ref%29))
  (bind _returnvalue (Game|GetPlayerController 0))
  (if (Actor|ActorHasTag OtherActor "Player")
    (bind _returnvalue_2 (UserInterface|CreateWidget "/Game/UI/UI_NarrativePopUp.UI_NarrativePopUp_C"))
    (Rendering|Components|TextRender|SetText (Variables|/Game/UI/UI_NarrativePopUp.UI_NarrativePopUp_C|GetNarrativeText _returnvalue_2) (Variables|Default|GetNarrativeText))
    (UserInterface|Viewport|AddtoViewport _returnvalue_2 0)
    (Input|DisableInput (Game|Player|GetPlayerPawn 0) _returnvalue)
    (Variables|/Script/Engine.PlayerController|SetbShowMouseCursor _returnvalue true)))

(event OnComponentEndOverlap(Box)
  (params (OverlappedComponent :type Primitive%20Component%20Object%20Reference) (OtherActor :type Actor%20Object%20Reference) (OtherComp :type Primitive%20Component%20Object%20Reference) (OtherBodyIndex :type Integer))
  (if (Actor|ActorHasTag OtherActor "Player")
    _))

(fn ConstructionScript)