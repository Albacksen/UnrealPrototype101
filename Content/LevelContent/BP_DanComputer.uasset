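; BP_DanComputer is an interactable computer in level content that can slide along a spline.
; Activation enables interaction, after which Interact prints a taunting line addressed to Dave.
; MoveComputer plays a timeline that places the Computer component along the spline in world space, without sweeping.
; The timeline value serves as both Lerp start and blend factor toward the spline length.
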(event Custom|MoveComputer
  (bind _newtrack_0 (Timeline|Timeline_0 PlayFromStart)
    (:Update
      (bind _output_get (Variables|Default|SetAlpha _newtrack_0))
      (Transformation|SetWorldLocation (Variables|Default|GetComputer) (Spline|GetLocationatDistanceAlongSpline (Variables|Default|GetSpline) (Math|Float|Lerp _output_get (Spline|GetSplineLength (Variables|Default|GetSpline)) (Variables|Default|GetAlpha)) "World") false false))))

(event Custom|Activation
  (Variables|Default|SetCanActivate true))

(event EventInteract
  (if (Variables|Default|GetCanActivate)
    (Development|PrintString "What do you thing you are doing Dave?")))

(fn ConstructionScript)